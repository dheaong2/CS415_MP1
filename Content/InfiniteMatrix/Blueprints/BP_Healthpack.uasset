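; BP_Healthpack is a spinning health pickup that restores a fixed amount of the player's health.
; Tick applies a frame-rate independent yaw spin to the actor.
; When BP_Player overlaps the Box, it adds health capped at the maximum, refreshes the player's health bar widget and destroys the pack.
; A BP_Projectile overlapping the Box is destroyed through its own DestroyProjectile, leaving the pack in place.
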(event OnComponentBeginOverlap(Box)
  (params (OverlappedComponent :type Primitive%20Component%20Object%20Reference) (OtherActor :type Actor%20Object%20Reference) (OtherComp :type Primitive%20Component%20Object%20Reference) (OtherBodyIndex :type Integer) (bFromSweep :type Boolean) (SweepResult :type Hit%20Result%20Structure%20%28by%20ref%29))
  (Utilities|FlowControl|Sequence
    (:then_0
      (bind _asbp_player (Utilities|Casting|CastToBP_Player OtherActor))
      (if (> (+ (Variables|/Game/InfiniteMatrix/Blueprints/BP_Player.BP_Player_C|GetPlayerHealth _asbp_player) 2e+01) 1e+02)
        (bind _output_get (Variables|/Game/InfiniteMatrix/Blueprints/BP_Player.BP_Player_C|SetPlayerHealth _asbp_player 1e+02))
        (Default|UpdateHealthBar (Variables|/Game/InfiniteMatrix/Blueprints/BP_Player.BP_Player_C|GetHealthWidget _asbp_player) _output_get)
        (Actor|DestroyActor)
        (else
          (bind _output_get_2 (Variables|/Game/InfiniteMatrix/Blueprints/BP_Player.BP_Player_C|SetPlayerHealth _asbp_player (+ (Variables|/Game/InfiniteMatrix/Blueprints/BP_Player.BP_Player_C|GetPlayerHealth _asbp_player) 2e+01)))
          (Default|UpdateHealthBar (Variables|/Game/InfiniteMatrix/Blueprints/BP_Player.BP_Player_C|GetHealthWidget _asbp_player) _output_get_2)
          (Actor|DestroyActor))))
    (:then_1
      (bind _asbp_projectile (Utilities|Casting|CastToBP_Projectile OtherActor))
      (Default|DestroyProjectile _asbp_projectile))))

(event EventBeginPlay)

(event Collision|EventActorBeginOverlap
  (params (OtherActor :type Actor%20Object%20Reference)))

(event EventTick
  (params (DeltaSeconds :type Float%20%28single-precision%29))
  (Transformation|AddActorLocalRotation (* (Math|Rotator|MakeRotator 0.0 0.0 2e+02) DeltaSeconds) false false))

(fn ConstructionScript)