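; BP_Enemy is a spinning enemy that hurts the player on contact and awards score when shot.
; It rotates on yaw every tick, and its box overlap handles both player and projectile hits.
; Touching BP_Player deducts health, updates the health widget and destroys the enemy, triggering death and the restart display at zero health.
; A BP_Projectile hit raises its owning player's score and widget, then destroys projectile and enemy.
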(event OnComponentBeginOverlap(Box)
  (params (OverlappedComponent :type Primitive%20Component%20Object%20Reference) (OtherActor :type Actor%20Object%20Reference) (OtherComp :type Primitive%20Component%20Object%20Reference) (OtherBodyIndex :type Integer) (bFromSweep :type Boolean) (SweepResult :type Hit%20Result%20Structure%20%28by%20ref%29))
  (Utilities|FlowControl|Sequence
    (:then_0
      (bind _asbp_player (Utilities|Casting|CastToBP_Player OtherActor))
      (bind _output_get (Variables|/Game/InfiniteMatrix/Blueprints/BP_Player.BP_Player_C|SetPlayerHealth _asbp_player (- (Variables|/Game/InfiniteMatrix/Blueprints/BP_Player.BP_Player_C|GetPlayerHealth _asbp_player) 1e+01)))
      (Default|UpdateHealthBar (Variables|/Game/InfiniteMatrix/Blueprints/BP_Player.BP_Player_C|GetHealthWidget _asbp_player) _output_get)
      (Actor|DestroyActor)
      (if (<= _output_get 0.0)
        (Variables|/Game/InfiniteMatrix/Blueprints/BP_Player.BP_Player_C|SetIsDead _asbp_player true)
        (Default|DisplayRestart _asbp_player)))
    (:then_1
      (bind _asbp_projectile (Utilities|Casting|CastToBP_Projectile OtherActor))
      (bind _output_get_2 (Variables|/Game/InfiniteMatrix/Blueprints/BP_Player.BP_Player_C|SetPlayerScore (Variables|/Game/InfiniteMatrix/Blueprints/BP_Projectile.BP_Projectile_C|GetRefPlayer _asbp_projectile) (+ (Variables|/Game/InfiniteMatrix/Blueprints/BP_Player.BP_Player_C|GetPlayerScore (Variables|/Game/InfiniteMatrix/Blueprints/BP_Projectile.BP_Projectile_C|GetRefPlayer _asbp_projectile)) 1)))
      (Default|UpdatePlayerScore (Variables|/Game/InfiniteMatrix/Blueprints/BP_Player.BP_Player_C|GetScoreWidget (Variables|/Game/InfiniteMatrix/Blueprints/BP_Projectile.BP_Projectile_C|GetRefPlayer _asbp_projectile)) _output_get_2)
      (Actor|DestroyActor _asbp_projectile)
      (Actor|DestroyActor))))

(event EventBeginPlay)

(event Collision|EventActorBeginOverlap
  (params (OtherActor :type Actor%20Object%20Reference)))

(event EventTick
  (params (DeltaSeconds :type Float%20%28single-precision%29))
  (Transformation|AddActorLocalRotation (* (Math|Rotator|MakeRotator 0.0 0.0 1e+02) DeltaSeconds) false false))

(fn ConstructionScript)